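; Actor that drives a Niagara echo effect of a skeletal mesh, using copies of a base-pose static mesh.
; Construction validates inputs, creates body and hair dynamic materials, then passes them, both meshes, echo settings and render targets to Niagara.
; Niagara and both materials share position and normal render targets plus frame layout, suggesting texture-based vertex animation.
; BeginPlay resends the Niagara parameters, while Tick updates only location spacing.
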(event EventBeginPlay
  (CallFunction|InitializeNiagaraParams))

(event EventTick
  (params (DeltaSeconds :type Float%20%28single-precision%29))
  (CallFunction|NiagaraUpdateParams))

(fn ConstructionScript
  (CallFunction|Initialize))

(fn InitializeNiagaraParams
  (Class|NiagaraComponent|SetVariableInt (Variables|Default|GetNS_EchoEffect) "FrameSize" (Variables|Settings|GetFrameSize))
  (Class|NiagaraComponent|SetVariableInt (Variables|Default|GetNS_EchoEffect) "EchoSpacing" (Variables|Settings|GetEchoSpacing))
  (Class|NiagaraComponent|SetVariableInt (Variables|Default|GetNS_EchoEffect) "TextureWidth" (Variables|Settings|GetTextureResolutionX))
  (Class|NiagaraComponent|SetVariableInt (Variables|Default|GetNS_EchoEffect) "TextureHeight" (Variables|Settings|GetTextureResolutionY))
  (Class|NiagaraComponent|SetVariableTextureRenderTarget (Variables|Default|GetNS_EchoEffect) "RT_Positions" (Variables|Data|GetPositionsTexture))
  (Class|NiagaraComponent|SetVariableTextureRenderTarget (Variables|Default|GetNS_EchoEffect) "RT_Normals" (Variables|Data|GetNormalsTexture))
  (Class|NiagaraFunctionLibrary|OverrideSystemUserVariableSkeletalMeshComponent (Variables|Default|GetNS_EchoEffect) "SkeletalMesh" (Variables|/Script/Engine.SkeletalMeshActor|GetSkeletalMeshComponent (Variables|Data|GetSkeletalMesh)))
  (Class|NiagaraComponent|SetVariableStaticMesh (Variables|Default|GetNS_EchoEffect) "StaticMesh" (Variables|Data|GetBasePoseMesh))
  (Class|NiagaraComponent|SetVariableInt (Variables|Default|GetNS_EchoEffect) "EchoCount" (Variables|Settings|GetEchoCount))
  (Utilities|FlowControl|Sequence
    (:then_0
      (bind _dmi_body (Variables|Data|GetDMI_Body)
        (:then
          (Class|NiagaraComponent|SetVariableMaterial (Variables|Default|GetNS_EchoEffect) "BodyMaterial" _dmi_body))
        (:else)))
    (:then_1
      (bind _dmi_hair (Variables|Data|GetDMI_Hair)
        (:then
          (Class|NiagaraComponent|SetVariableMaterial (Variables|Default|GetNS_EchoEffect) "HairMaterial" _dmi_hair))
        (:else)))))

(fn CreateEchoMaterial
  (Utilities|FlowControl|Sequence
    (:then_0
      (bind _returnvalue (Rendering|Material|CreateDynamicMaterialInstance (Variables|Data|GetEchoMaterialBody) "BodyEchoMaterial" "None" :!class /Script/Engine.KismetMaterialLibrary))
      (Variables|Data|SetDMI_Body _returnvalue)
      (bind _returnvalue_2 (Rendering|Material|CreateDynamicMaterialInstance (Variables|Data|GetEchoMaterialHair) "HairEchoMaterial" "None" :!class /Script/Engine.KismetMaterialLibrary))
      (Variables|Data|SetDMI_Hair _returnvalue_2))
    (:then_1
      (CallFunction|SetDynamicMaterialInstanceParams (Variables|Data|GetDMI_Body))
      (CallFunction|SetDynamicMaterialInstanceParams (Variables|Data|GetDMI_Hair)))))

(fn Initialize
  (if (Math|Boolean|ANDBoolean (Utilities|IsValid (Variables|Data|GetSkeletalMesh)) (Utilities|IsValid (Variables|Data|GetBasePoseMesh)) (> (* (Variables|Settings|GetTextureResolutionX) (Variables|Settings|GetTextureResolutionY) (Variables|Settings|GetFrameSize)) 0) (Utilities|IsValid (Variables|Data|GetPositionsTexture)) (Utilities|IsValid (Variables|Data|GetNormalsTexture)))
    (CallFunction|CreateEchoMaterial)
    (CallFunction|InitializeNiagaraParams)
    (CallFunction|NiagaraUpdateParams)))

(fn NiagaraUpdateParams
  (Niagara|SetNiagaraVariable(Vector3) (Variables|Default|GetNS_EchoEffect) "LocationSpacing" (Variables|Settings|GetLocationSpacing)))

(fn SetDynamicMaterialInstanceParams
  (params (Target :type Material%20Instance%20Dynamic%20Object%20Reference))
  (Rendering|Material|SetScalarParameterValue Target "FrameSize" (Math|Conversions|ToFloat(Integer) (Variables|Settings|GetFrameSize)) :!class /Script/Engine.MaterialInstanceDynamic)
  (Rendering|Material|SetScalarParameterValue Target "TextureResolutionX" (Math|Conversions|ToFloat(Integer) (Variables|Settings|GetTextureResolutionX)) :!class /Script/Engine.MaterialInstanceDynamic)
  (Rendering|Material|SetScalarParameterValue Target "TextureResolutionY" (Math|Conversions|ToFloat(Integer) (Variables|Settings|GetTextureResolutionY)) :!class /Script/Engine.MaterialInstanceDynamic)
  (Rendering|Material|SetTextureParameterValue Target "PositionsTexture" (Variables|Data|GetPositionsTexture))
  (Rendering|Material|SetTextureParameterValue Target "NormalsTexture" (Variables|Data|GetNormalsTexture)))